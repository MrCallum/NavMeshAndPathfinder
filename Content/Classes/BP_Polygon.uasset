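; BP_Polygon is a single 2D navmesh triangle, storing its corners, bounding box, centroid and neighbour indices.
; SetCoords derives the box and centroid, and AdjustCoords feeds it voxel coordinates converted to world-space voxel centres.
; Neighbour tests match identical vertices, with exactly two meaning a shared edge.
; Point-in-triangle compares angles and cross-product signs at two corners, optionally expanding the triangle from its centroid to tolerate near misses during corridor clipping.
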(fn `AddNeighbourIndex`
  (params (neighbourIndex :type Integer))
  (`KismetArrayLibrary.Array_AddUnique` (`self.neighbourIndecies`) neighbourIndex))

(fn `AdjustCoords`
  (params (voxelLength :type "Float (double-precision)") (navBoundTopLeft :type "Vector Structure"))
  (locals (xVoxelAddition :type "Float (double-precision)") (yVoxelAddition :type "Float (double-precision)") (coordsCopy :type "Array of Vector2D Structure"))
  (bind _voxellength (`local.voxelLength`))
  (bind _coords (`self.Coords`))
  (bind _returnvalue (/ (`local.voxelLength`) 2.0))
  (`KismetArrayLibrary.Array_Resize` (`local.coordsCopy`) (`KismetArrayLibrary.Array_Length` (`self.Coords`)))
  (for _index (range (+ (`KismetArrayLibrary.Array_LastIndex` _coords) 1))
    (bind (_x _y) (`KismetMathLibrary.BreakVector2D` (`|GetArrayItem` _coords _index)))
    (set `local.xVoxelAddition` (* _x _voxellength))
    (set `local.yVoxelAddition` (* _y _voxellength))
    ;[1 1 1] Add real world coord to buffer
    (`KismetArrayLibrary.Array_Set` (`local.coordsCopy`) _index (`KismetMathLibrary.MakeVector2D` (+ (.x (`local.navBoundTopLeft`)) _returnvalue (`local.xVoxelAddition`)) (+ (.y (`local.navBoundTopLeft`)) _returnvalue (`local.yVoxelAddition`)))))
  ;[0.2392 1 0.9781] Commit these new coords
  (`self.SetCoords` (`local.coordsCopy`)))

(fn `CalculateAngleFromPoints`
  (params (left :type "Vector2D Structure") (center :type "Vector2D Structure") (right :type "Vector2D Structure"))
  (returns (degrees :type "Float (double-precision)"))
  (bind _returnvalue (- right center))
  (bind _returnvalue_2 (- left center))
  (return (`KismetMathLibrary.DegAcos` (/ (`KismetMathLibrary.DotProduct2D` _returnvalue_2 _returnvalue) (* (`KismetMathLibrary.VSize2D` _returnvalue_2) (`KismetMathLibrary.VSize2D` _returnvalue))))))

(fn `CalculateCentroid`
  (returns (centroid :type "Vector2D Structure"))
  (locals (midpointAB :type "Vector2D Structure"))
  (bind _coords (`self.Coords`))
  (bind _output (`|GetArrayItem` _coords 2))
  (bind _output_2 (`|GetArrayItem` _coords))
  (bind _returnvalue (/ 2.0 3.0))
  (bind _output_get (set `local.midpointAB` (+ _output_2 (/ (- (`|GetArrayItem` _coords 1) _output_2) (2.0 2.0)))))
  (return (+ _output (* (- _output_get _output) (`KismetMathLibrary.MakeVector2D` _returnvalue _returnvalue)))))

(fn `CallumPoliesShareEdge`
  (params (potentialNeighbour :type "/Game/Classes/BP_Polygon Object Reference"))
  (returns (EdgeShared :type Boolean))
  (locals (sharedVertecies :type Integer))
  (bind _coords (`self.Coords`))
  (for _array_element (`/Game/Classes/BP_Polygon.Coords` potentialNeighbour)
    (for _index (range (+ (`KismetArrayLibrary.Array_LastIndex` _coords) 1))
      (if (`KismetMathLibrary.EqualExactly_Vector2DVector2D` _array_element (`|GetArrayItem` _coords _index))
        (`/Engine/EditorBlueprintResources/StandardMacros.IncrementInt` (`local.sharedVertecies`)))))
  (return (== (`local.sharedVertecies`) 2)))

(fn `GetCoords`
  (returns (Coords :type "Array of Vector2D Structure"))
  (return (`self.Coords`)))

(fn `GetCrossProduct`
  (params (left :type "Vector2D Structure") (centre :type "Vector2D Structure") (right :type "Vector2D Structure"))
  (returns (ReturnValue :type Boolean))
  (return (< (`KismetMathLibrary.CrossProduct2D` (- left centre) (- right centre)) 0.0)))

(fn `GetSharedVerticies`
  (params (neighbour :type "/Game/Classes/BP_Polygon Object Reference"))
  (returns (sharedVerticies :type "Array of Vector2D Structure"))
  (locals (sharedVerts :type "Array of Vector2D Structure"))
  (bind _coords (`self.Coords`))
  (for _array_element (`/Game/Classes/BP_Polygon.Coords` neighbour)
    (for _index (range (+ (`KismetArrayLibrary.Array_LastIndex` _coords) 1))
      (bind _output (`|GetArrayItem` _coords _index))
      (if (`KismetMathLibrary.EqualExactly_Vector2DVector2D` _array_element _output)
        (`KismetArrayLibrary.Array_Add` (`local.sharedVerts`) _output))))
  (return (`local.sharedVerts`)))

(fn `PointIsWithinThisPoly`
  (params (point :type "Vector2D Structure") (additionalExpandPercentage :type "Float (double-precision)"))
  (returns (pointIsInPoly :type Boolean))
  (locals (coord0 :type "Vector2D Structure") (coord1 :type "Vector2D Structure") (coord2 :type "Vector2D Structure"))
  (bind _point (`local.point`))
  (bind _point_2 (`local.point`))
  (bind _coord0 (`local.coord0`))
  (bind _coord1 (`local.coord1`))
  (bind _coord2 (`local.coord2`))
  (bind _coord0_2 (`local.coord0`))
  (bind _coord0_3 (`local.coord0`))
  (bind _coord1_2 (`local.coord1`))
  (bind _coord2_2 (`local.coord2`))
  (bind _coords (`self.Coords`))
  (bind _coord0_4 (`local.coord0`))
  (bind _coord1_3 (`local.coord1`))
  (bind _coord2_3 (`local.coord2`))
  (bind _output (`|GetArrayItem` _coords))
  (bind _output_2 (`|GetArrayItem` _coords 1))
  (bind _output_3 (`|GetArrayItem` _coords 2))
  (if (== additionalExpandPercentage 0.0)
    (set `local.coord0` _output)
    (set `local.coord1` _output_2)
    (set `local.coord2` _output_3)
    (else
      ;[1 0.5757 0.8967] Used in vertex corrdior clipping. In certain situations a vertex would be super close to a poly but not quite in it which would mean the poly gets clipped when it probably shouldn't be. Solved by making the poly for this pointInPoly check slightly bigger
      (set `local.coord0` (`self.PushCoordFurtherfromCentroid` additionalExpandPercentage _output))
      (set `local.coord1` (`self.PushCoordFurtherfromCentroid` additionalExpandPercentage _output_2))
      (set `local.coord2` (`self.PushCoordFurtherfromCentroid` additionalExpandPercentage _output_3))))
  (if (and (<= (`self.CalculateAngleFromPoints` _coord0_4 _coord1_3 _point_2) (`self.CalculateAngleFromPoints` _coord0_3 _coord1_2 _coord2_2)) (== (`self.GetCrossProduct` _coord0_3 _coord1_2 _coord2_2) (`self.GetCrossProduct` _coord0_4 _coord1_3 _point_2)))
    (return (and (<= (`self.CalculateAngleFromPoints` _coord2_3 _coord0 _point) (`self.CalculateAngleFromPoints` _coord2 _coord0_2 _coord1)) (== (`self.GetCrossProduct` _coord2 _coord0_2 _coord1) (`self.GetCrossProduct` _coord2_3 _coord0 _point))))
    (else
      (return false))))

(fn `PointWithinPolyBoundingBox`
  (params (point :type "Vector2D Structure"))
  (returns (PointInBounds :type Boolean))
  (bind (_x _y) (`KismetMathLibrary.BreakVector2D` point))
  (bind (_min _max) (break `Box2D` (`self.boundingBox`)))
  (bind (_x_2 _y_2) (`KismetMathLibrary.BreakVector2D` _min))
  (bind (_x_3 _y_3) (`KismetMathLibrary.BreakVector2D` _max))
  (return (and (`KismetMathLibrary.InRange_FloatFloat` _x _x_2 _x_3) (`KismetMathLibrary.InRange_FloatFloat` _y _y_2 _y_3))))

(fn `PolyOverlapsBoundingBox`
  (params (boundingBox :type "Box2D Structure"))
  (returns (overlap :type Boolean))
  (bind (_min _max) (break `Box2D` boundingBox))
  (bind (_x _y) (`KismetMathLibrary.BreakVector2D` _max))
  (bind (_x_2 _y_2) (`KismetMathLibrary.BreakVector2D` _min))
  (for _array_element (`self.Coords`)
    (bind (_x_3 _y_3) (`KismetMathLibrary.BreakVector2D` _array_element))
    (if (and (`KismetMathLibrary.InRange_FloatFloat` _x_3 _x_2 _x) (`KismetMathLibrary.InRange_FloatFloat` _y_3 _y_2 _y))
      (return true)))
  (return false))

(fn `PushCoordFurtherfromCentroid`
  (params (extraPushOut :type "Float (double-precision)") (originalCoord :type "Vector2D Structure"))
  (returns (ReturnValue :type "Vector2D Structure"))
  (return (+ (`self.Centroid`) (* (- originalCoord (`self.Centroid`)) (+ extraPushOut 1.0)))))

(fn `SetCoords`
  (params (newCoords :type "Array of Vector2D Structure"))
  ;[1 1 1] Set coords and also calculate other values which will be useful later.
  (bind _output_get (set `self.Coords` newCoords))
  (bind (_x _y) (`KismetMathLibrary.BreakVector2D` (`|GetArrayItem` _output_get)))
  (bind (_x_2 _y_2) (`KismetMathLibrary.BreakVector2D` (`|GetArrayItem` _output_get 1)))
  (bind (_x_3 _y_3) (`KismetMathLibrary.BreakVector2D` (`|GetArrayItem` _output_get 2)))
  (set `self.boundingBox` (`KismetMathLibrary.MakeBox2D` (`KismetMathLibrary.MakeVector2D` (`KismetMathLibrary.FMin` _x _x_2 _x_3) (`KismetMathLibrary.FMin` _y _y_2 _y_3)) (`KismetMathLibrary.MakeVector2D` (`KismetMathLibrary.FMax` _x _x_2 _x_3) (`KismetMathLibrary.FMax` _y _y_2 _y_3))))
  (set `self.Centroid` (`self.CalculateCentroid`)))