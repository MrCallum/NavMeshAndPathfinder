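; BP_PolyMaker triangulates completed NavMesh perimeter chains into BP_Polygon triangles in relative coordinates, to be moved to world positions later.
; It derives each vertex's 90 or 270 degree angle from the hit grid cell at that corner.
; Ear clipping then repeatedly picks a triangle by most-acute or most-equal angles, rejects those containing reflex vertices, and updates neighbouring angles.
; Optional 180-degree vertex removal reduces polygon count but is noted as buggy.
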(event `ReadMe`
  ;[1 1 1] This class works with relative coordinates and will create polies with relative coordinates.
  ;
  ; All the polies created will later need to be adjusted to their real world positions
)

(fn `CalculateAdjustment`
  (params (pivotPoint :type "Vector2D Structure") (neighbourPoint :type "Vector2D Structure"))
  (returns (adjustment :type "Vector2D Structure"))
  (bind (_x _y) (`KismetMathLibrary.BreakVector2D` neighbourPoint))
  (bind (_x_2 _y_2) (`KismetMathLibrary.BreakVector2D` pivotPoint))
  ;[1 1 1] chain moves left (towards 0 x)
  (if (> _x _x_2)
    ;[0.8253 0.5268 1 1 16] Take half a step in the direction the chain moves
    (return (0.5 0.0))
    (else
      ;[1 1 1] right (away from 0 X)
      (if (< _x _x_2)
        (return (-0.5 0.0))
        (else
          ;[1 1 1] Up (back to 0 y)
          (if (> _y _y_2)
            (return (0.0 0.5))
            (else
              (return (0.0 -0.5)))))))))

(fn `CalculateAngleFromPoints`
  (params (left :type "Vector2D Structure") (center :type "Vector2D Structure") (right :type "Vector2D Structure"))
  (returns (degrees :type "Float (double-precision)"))
  (bind _returnvalue (- right center))
  (bind _returnvalue_2 (- left center))
  (return (`KismetMathLibrary.DegAcos` (/ (`KismetMathLibrary.DotProduct2D` _returnvalue_2 _returnvalue) (* (`KismetMathLibrary.VSize2D` _returnvalue_2) (`KismetMathLibrary.VSize2D` _returnvalue))))))

(fn `CalculateCornerCellFromPoints`
  (params (previousCoord :type "Vector2D Structure") (centreCoord :type "Vector2D Structure") (nextCoord :type "Vector2D Structure"))
  (returns (centreCell :type "Vector2D Structure"))
  (return (+ centreCoord (`self.CalculateAdjustment` centreCoord previousCoord) (`self.CalculateAdjustment` centreCoord nextCoord))))

(fn `ClipInteriorIntoPolies`
  (params (chain :type "/Game/Structs/ST_CoordChain Structure") (triangulationMethod :type "/Game/Structs/Enum_TriangulationMethod Enum" :default "NewEnumerator0") (allow180Clipping :type Boolean))
  (returns (newStylePolies1 :type "Array of /Game/Classes/BP_Polygon Object Reference") (outstandingPoints1 :type "Array of Vector2D Structure"))
  (locals (outstandingPoints :type "Array of Vector2D Structure") (angles :type "Array of Float (double-precision)") (smallestPolyIndex :type Integer) (previousIndex :type Integer) (currentIndex :type Integer) (nextIndex :type Integer) (thisLeftAngle :type "Float (double-precision)" :default 0.0) (thisCentreAngle :type "Float (double-precision)") (thisRightAngle :type "Float (double-precision)") (smallestPolyAngles :type "Vector Structure") (newStylePolies :type "Array of /Game/Classes/BP_Polygon Object Reference") (newStyleCurrentSmallestPoly :type "/Game/Classes/BP_Polygon Object Reference"))
  (bind _angles (`local.angles`))
  (bind _angles_2 (`local.angles`))
  (bind _previousindex (`local.previousIndex`))
  (bind (_smallestpolyangles_x _smallestpolyangles_y _smallestpolyangles_z) (`KismetMathLibrary.BreakVector` (`local.smallestPolyAngles`)))
  (bind _nextindex (`local.nextIndex`))
  (bind _currentindex (`local.currentIndex`))
  (bind _outstandingpoints (`local.outstandingPoints`))
  (set `self.Triangulation Method` triangulationMethod)
  (`|ExecutionSequence`
    (:`then_0`
      (bind _angles1 (`self.ProcessChainIntoInitialVerticies` chain))
      ;[1 1 1] A map would have been nice but the order is important, so a map is not sufficient.
      (set `local.angles` _angles1)
      (set `local.outstandingPoints` (`.coordinates_7_292AFAFC46D8A9CB612BF7A4E4CAFF15` (break `/Game/Structs/ST_CoordChain` chain))))
    (:`then_1`
      (bind _returnvalue (`|GenericCreateObject` "/Game/Classes/BP_Polygon.BP_Polygon_C"))
      (set `local.newStyleCurrentSmallestPoly` _returnvalue))
    (:`then_2`
      ;[0.575 1 0.461 1 16] While their are still oustanding points (from the original perimeter), we loop through all potential polies.
      ; Of the potential polies, we get one that is "best".
      ; This best poly has one vertex that is being "clipped" from the reaminging NavMesh. IE we remove one element from the oustanding points.
      (while (> (`KismetArrayLibrary.Array_Length` (`local.outstandingPoints`)) 3)
        (`|ExecutionSequence`
          (:`then_0`
            ;[1 1 1] Reset
            (set `local.smallestPolyAngles` (360.0 360.0 360.0))
            (set `local.smallestPolyIndex` -1))
          (:`then_1`
            ;[1 1 1] Loop through all the oustanding points and evaluate what poly each point could be used for. Record the "best" one,
            (for _index (range (+ (`KismetArrayLibrary.Array_LastIndex` (`local.outstandingPoints`)) 1))
              (set `local.currentIndex` _index)
              (`self.ProgressIndecies` (`local.previousIndex`) (`local.nextIndex`) (`local.currentIndex`) (`local.outstandingPoints`))
              (bind (_newpolyisbetter _coords _newsmallestangles) (`self.EvaluatePotentialPoly` (`local.angles`) (`local.currentIndex`) (`local.previousIndex`) (`local.nextIndex`) (`local.outstandingPoints`) (`local.smallestPolyAngles`)))
              ;;[1 1 1] This potential poly is, so far, the "best" we have found. Record it.
              (if _newpolyisbetter
                (`/Game/Classes/BP_Polygon.SetCoords` (`local.newStyleCurrentSmallestPoly`) _coords)
                (set `local.smallestPolyAngles` _newsmallestangles)
                (set `local.smallestPolyIndex` (`local.currentIndex`))))
            (if (!= (`local.smallestPolyIndex`) -1)
              ;[1 1 1] Best poly has been found. Do the following:
              ; 1 - add this poly to our list of polies.
              ; 2 - Two of the three points used to make this poly are still in use -> update their angles to relfect how much they just changed,
              ; 3 - Remove the point and associated angle that has been "clipped off" from "oustanding points" and "angles" arrays.
              (set `local.currentIndex` (`local.smallestPolyIndex`))
              (`|ExecutionSequence`
                (:`then_0`
                  (`self.ProgressIndecies` (`local.previousIndex`) (`local.nextIndex`) (`local.currentIndex`) (`local.outstandingPoints`)))
                (:`then_1`
                  (bind _returnvalue_2 (`|GenericCreateObject` "/Game/Classes/BP_Polygon.BP_Polygon_C"))
                  (`/Game/Classes/BP_Polygon.SetCoords` _returnvalue_2 (`/Game/Classes/BP_Polygon.GetCoords` (`local.newStyleCurrentSmallestPoly`)))
                  (`KismetArrayLibrary.Array_Add` (`local.newStylePolies`) _returnvalue_2))
                (:`then_2`
                  ;[0.581 1 0.7565] Update the left and right angles. IE subtract the angle that was just clipped off. Remove the clipped vertex from the oustanding list of vertexes and angles.
                  (`KismetArrayLibrary.Array_Set` _angles_2 _previousindex (- (`|GetArrayItem` _angles_2 _previousindex) _smallestpolyangles_x))
                  (`KismetArrayLibrary.Array_Set` _angles _nextindex (- (`|GetArrayItem` _angles _nextindex) _smallestpolyangles_z))
                  (`KismetArrayLibrary.Array_Remove` (`local.outstandingPoints`) _currentindex)
                  (`KismetArrayLibrary.Array_Remove` (`local.angles`) _currentindex)
                  (if (`local.allow180Clipping`)
                    ;[1 1 1] This allowed 180 deg angles to be auto removed. It leads to fewer polies but has more bugs.
                    ; But I don't think it should be allowed as it means a single poly edge can have any number of neighbours (think of a shape like the letter E: one triangle could border every arm of the E). This will lead to problems when trying to determine which polies are connected.
                    (bind (_arrayindex _arrayelement) (`/Engine/EditorBlueprintResources/StandardMacros.ReverseForEachLoop` (`local.angles`))
                      (:`LoopBody`
                        (if (== _arrayelement 180.0)
                          (`KismetArrayLibrary.Array_Remove` (`local.angles`) _arrayindex)
                          (`KismetArrayLibrary.Array_Remove` (`local.outstandingPoints`) _arrayindex)))))))
              (else
                ;[1 0.09883 0] This should never happen in theory.
                (`KismetSystemLibrary.PrintString` null "Warning! Could not find any more potential polies!")
                (if (`self.triangulationHasBeenReattempted`)
                  (return (`local.newStylePolies`) (`local.outstandingPoints`))
                  (else
                    (set `self.triangulationHasBeenReattempted` true))))))))
      ;[1 1 1] Add the last available poly.
      (bind _returnvalue_3 (`|GenericCreateObject` "/Game/Classes/BP_Polygon.BP_Polygon_C"))
      (`/Game/Classes/BP_Polygon.SetCoords` _returnvalue_3 (`|MakeArray` (`|GetArrayItem` _outstandingpoints) (`|GetArrayItem` _outstandingpoints 1) (`|GetArrayItem` _outstandingpoints 2)))
      (`KismetArrayLibrary.Array_Add` (`local.newStylePolies`) _returnvalue_3)
      ;[0.4326 1 0.3972] Finished and successful. Return all polies.
      (return (`local.newStylePolies`)))))

(fn `EvaluatePotentialPoly`
  (params (Angles :type "Array of Float (double-precision)") (currIndex :type Integer) (prevIndex :type Integer) (nexIndex :type Integer) (outstandingPoints :type "Array of Vector2D Structure") (previousSmallestAngles :type "Vector Structure"))
  (returns (newPolyIsBetter :type Boolean) (coords :type "Array of Vector2D Structure") (newSmallestAngles :type "Vector Structure"))
  (locals (angles :type "Array of Float (double-precision)") (thisCentreAngle :type "Float (double-precision)") (thisLeftAngle :type "Float (double-precision)") (thisRightAngle :type "Float (double-precision)") (foundVertexInPoly :type Boolean) (currentPoly :type "/Game/Classes/BP_Polygon Object Reference"))
  (bind (_previoussmallestangles_x _previoussmallestangles_y _previoussmallestangles_z) (`KismetMathLibrary.BreakVector` (`local.previousSmallestAngles`)))
  (bind _outstandingpoints (`local.outstandingPoints`))
  (bind _previoussmallestangles_x_2 (`KismetMathLibrary.BreakVector` (`local.previousSmallestAngles`)))
  (bind _outstandingpoints_2 (`local.outstandingPoints`))
  (bind _thisleftangle (`local.thisLeftAngle`))
  (bind _thiscentreangle (`local.thisCentreAngle`))
  (bind _thisrightangle (`local.thisRightAngle`))
  (bind (_previoussmallestangles_x_3 _previoussmallestangles_y_2 _previoussmallestangles_z_2) (`KismetMathLibrary.BreakVector` (`local.previousSmallestAngles`)))
  (bind _coords (`/Game/Classes/BP_Polygon.GetCoords` (`local.currentPoly`)))
  (bind _returnvalue (`KismetMathLibrary.FMin` (`local.thisLeftAngle`) (`local.thisCentreAngle`) (`local.thisRightAngle`)))
  (`|ExecutionSequence`
    (:`then_0`
      ;[1 1 1] Only consider this point for a poly if it is not reflexive.
      (bind _output_get (set `local.thisCentreAngle` (`|GetArrayItem` (`local.Angles`) (`local.currIndex`))))
      (if (not (< _output_get 180.0))
        (return false _ (0.0 0.0 0.0))))
    (:`then_1`
      ;[0.6544 0.9661 1] Find the next poly to clip
      ;;[1 0.8969 0.4299 1 16] Calculate the other two angles that would be made if we created a poly with verts i, i+1 and i-1.
      ;;
      ;; We know the angle at vertex i already.
      ;; Now we just need to calculate one angle, and then the remaining one is just 180 - angle 1 - angle 2.
      (bind _output_get_2 (set `local.thisLeftAngle` (`self.CalculateAngleFromPoints` (`|GetArrayItem` _outstandingpoints_2 (`local.currIndex`)) (`|GetArrayItem` _outstandingpoints_2 (`local.prevIndex`)) (`|GetArrayItem` _outstandingpoints_2 (`local.nexIndex`)))))
      (set `local.thisRightAngle` (- 180.0 _output_get_2 (`local.thisCentreAngle`)))
      (switch `/Game/Structs/Enum_TriangulationMethod` (`self.Triangulation Method`)
        (:`NewEnumerator0`
          ;[1 0.6426 0.3986] If this poly contained the smallest angle found so far (that isn't a straight line) -> investigate further to see if it is valid and potentially record it as the most acute poly we have found so far.
          (if (and (> _returnvalue 0.0) (< _returnvalue (`KismetMathLibrary.FMin` _previoussmallestangles_x_3 _previoussmallestangles_y_2 _previoussmallestangles_z_2)))
            _
            (else
              (return false _ (0.0 0.0 0.0)))))
        (:`NewEnumerator1`
          (if (== _previoussmallestangles_x_2 360.0)
            _
            (elif (< (- (`KismetMathLibrary.FMax` _thisleftangle _thiscentreangle _thisrightangle) (`KismetMathLibrary.FMin` _thisleftangle _thiscentreangle _thisrightangle)) (- (`KismetMathLibrary.FMax` _previoussmallestangles_x _previoussmallestangles_y _previoussmallestangles_z) (`KismetMathLibrary.FMin` _previoussmallestangles_x _previoussmallestangles_y _previoussmallestangles_z)))
              _
              (else
                (return false _ (0.0 0.0 0.0)))))))
      ;[1 1 1] make interim poly
      (bind _returnvalue_2 (`|GenericCreateObject` "/Game/Classes/BP_Polygon.BP_Polygon_C"))
      (bind _output_get_3 (set `local.currentPoly` _returnvalue_2))
      (`/Game/Classes/BP_Polygon.SetCoords` _output_get_3 (`|MakeArray` (`|GetArrayItem` _outstandingpoints (`local.prevIndex`)) (`|GetArrayItem` _outstandingpoints (`local.currIndex`)) (`|GetArrayItem` _outstandingpoints (`local.nexIndex`))))
      ;[1 1 1] Check all reflexive edges to see if they protrude into this potential current-best polygon.
      (set `local.foundVertexInPoly` false)
      (for (_array_element _array_index) (`local.Angles`)
        ;;[0.3962 1 0.8573] Only check reflexive point.
        (if (>= _array_element 180.0)
          (if (and (!= _array_index (`local.prevIndex`)) (!= _array_index (`local.currIndex`)) (!= _array_index (`local.nexIndex`)))
            (bind _output (`|GetArrayItem` (`local.outstandingPoints`) _array_index))
            ;;[1 0.6378 0.9518] Cheap check of whether this point is in the general range of the poly.
            (if (`/Game/Classes/BP_Polygon.PointWithinPolyBoundingBox` (`local.currentPoly`) _output)
              ;;[1 1 1] Expensive, but accurate & necessary check
              (if (`/Game/Classes/BP_Polygon.PointIsWithinThisPoly` (`local.currentPoly`) _output 0.0)
                (set `local.foundVertexInPoly` true)
                (if (`self.triangulationHasBeenReattempted`)
                  (`KismetSystemLibrary.PrintString` null (`KismetStringLibrary.Concat_StrStr` "Was looking at " (`KismetStringLibrary.Concat_StrStr` (`KismetStringLibrary.Conv_IntToString` (`local.prevIndex`)) "-" (`KismetStringLibrary.Conv_IntToString` (`local.currIndex`)) "-" (`KismetStringLibrary.Conv_IntToString` (`local.nexIndex`))) ". It had coords " (`KismetStringLibrary.Concat_StrStr` "[" (`KismetStringLibrary.Conv_Vector2dToString` (`|GetArrayItem` _coords)) "," (`KismetStringLibrary.Conv_Vector2dToString` (`|GetArrayItem` _coords 1)) "," (`KismetStringLibrary.Conv_Vector2dToString` (`|GetArrayItem` _coords 2)) "]") ". It couldn't be used though as the point with index " (`KismetStringLibrary.Conv_IntToString` _array_index) " is in the poly. It has coords " (`KismetStringLibrary.Conv_Vector2dToString` (`|GetArrayItem` (`local.outstandingPoints`) _array_index)) "."))
                  (else
                    (break))))))))
      (if (`local.foundVertexInPoly`)
        (return false _ (0.0 0.0 0.0))
        (else
          ;[0.5077 1 0.5142] We have found a new "most acute" poly. Record it in "potential poly" and record some info about it.
          (return true (`/Game/Classes/BP_Polygon.GetCoords` (`local.currentPoly`)) (`KismetMathLibrary.MakeVector` (`local.thisLeftAngle`) (`local.thisCentreAngle`) (`local.thisRightAngle`))))))))

(fn `GetAngleAtIndex`
  (params (Array :type "Array of Vector2D Structure") (index :type Integer))
  (returns (angle :type "Float (double-precision)"))
  (locals (previousIndex :type Integer :default 1) (nextIndex :type Integer))
  (bind _returnvalue (- index 1))
  (bind (_x _y) (`KismetMathLibrary.BreakVector2D` (`self.CalculateCornerCellFromPoints` (`|GetArrayItem` Array (`local.previousIndex`)) (`|GetArrayItem` Array index) (`|GetArrayItem` Array (`local.nextIndex`)))))
  ;[1 1 1] Seem % can't handle negative numbers
  (set `local.previousIndex` (`KismetMathLibrary.SelectInt` _returnvalue (`KismetArrayLibrary.Array_LastIndex` Array) (>= _returnvalue 0)))
  (set `local.nextIndex` (mod (+ index 1) (`KismetArrayLibrary.Array_Length` Array)))
  (return (`KismetMathLibrary.SelectFloat` 90.0 270.0 (`|GetArrayItem` (`self.Filtered Hit Data`) (`self.PolyMaker_2dTo1d` (`KismetMathLibrary.FTrunc` _x) (`KismetMathLibrary.FTrunc` _y))))))

(fn `Init`
  (params (filteredHitData :type "Array of Boolean") (`2dArrayWidth` :type Integer) (traingulationMethod :type "/Game/Structs/Enum_TriangulationMethod Enum" :default "NewEnumerator0"))
  ;[1 0.4819 0.5397] We init this object with the cell hit data but not the NavMesh perimeters.
  ;
  ; This is because we need the hit data in a few functions and it is handy to have it at hand rather than having to be passed in. The single set of hit data is used across all perimeter chains.
  ;
  ; As for the perimeter chains, these are processed individually and so are supplied and processed individually.
  ;
  ; This might be refactored.
  (set `self.Filtered Hit Data` filteredHitData)
  (set `self.2dArrayWidth` `2dArrayWidth`))

(fn `PolyMaker_2dTo1d`
  (params (x :type Integer) (y :type Integer))
  (returns (ReturnValue :type Integer))
  (return (+ x (* y (`self.2dArrayWidth`)))))

(fn `ProcessChainIntoInitialVerticies`
  (params (chain :type "/Game/Structs/ST_CoordChain Structure"))
  (returns (angles1 :type "Array of Float (double-precision)"))
  (locals (coordChain :type "Array of Vector2D Structure") (angles :type "Array of Float (double-precision)"))
  (bind (_coordinates _complete) (break `/Game/Structs/ST_CoordChain` chain))
  (if _complete
    (bind _output_get (set `local.coordChain` _coordinates))
    (`KismetArrayLibrary.Array_Resize` (`local.angles`) (`KismetArrayLibrary.Array_Length` _output_get))
    (for _index (range (+ (`KismetArrayLibrary.Array_LastIndex` (`local.coordChain`)) 1))
      (bind _angle (`self.GetAngleAtIndex` (`local.coordChain`) _index))
      (`KismetArrayLibrary.Array_Set` (`local.angles`) _index _angle))
    (return (`local.angles`))
    (else
      (`KismetSystemLibrary.PrintString` null "Warning! Chain supplied to \"Process Chain Into Initial Verticies\" is not \"complete\". It cannot be processed."))))

(fn `ProgressIndecies`
  (params (previousIndex :type "Integer (by ref)") (nextIndex :type "Integer (by ref)") (currentIndex :type Integer) (outstandingPoints :type "Array of Vector2D Structure"))
  (bind _returnvalue (- currentIndex 1))
  (`|VariableSetRef` previousIndex (`KismetMathLibrary.SelectInt` _returnvalue (`KismetArrayLibrary.Array_LastIndex` outstandingPoints) (>= _returnvalue 0)))
  (`|VariableSetRef` nextIndex (mod (+ currentIndex 1) (`KismetArrayLibrary.Array_Length` outstandingPoints))))