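; Navigation bounds volume that samples static geometry on a flat, axis-aligned voxel grid as raw data for a custom navmesh.
; SetUp derives cell counts and a corner origin from the Box component.
; RunVoxelCollisionChecks box-overlaps WorldStatic at each cell centre, storing hits row-major in RawVoxelHitData.
; Debug functions draw the grid, coordinates, raw or filtered cells and supplied triangles; filtering, triangle generation and calls to these functions lie outside this Blueprint.
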(fn `Debug Draw new style polies`
  (params (NewParam :type "Array of /Game/Classes/BP_Polygon Object Reference"))
  (locals (randomColour :type "LinearColor Structure" :default (struct :`R` 1.0 :`B` 0.790195 :`A` 1.0)) (colourPallet :type "Array of LinearColor Structure") (poly :type "/Game/Classes/BP_Polygon Object Reference"))
  (bind _randomcolour (`local.randomColour`))
  (bind _arrow_thickness (`self.Arrow Thickness`))
  (bind _arrow_size (`self.Arrow Size`))
  (bind _debugdrawduration (`self.debugDrawDuration`))
  (bind _colourpallet (`local.colourPallet`))
  (for (_array_element _array_index) NewParam
    (set `local.randomColour` (`|GetArrayItem` _colourpallet (mod _array_index (`KismetArrayLibrary.Array_Length` _colourpallet))))
    (bind _output_get (set `local.poly` _array_element))
    (bind _coords (`/Game/Classes/BP_Polygon.GetCoords` _output_get))
    (bind _returnvalue (`KismetMathLibrary.MakeVector` 0.0 0.0 (+ 100.0 (* _array_index 25.0))))
    (bind _returnvalue_2 (+ (`|GetArrayItem` _coords 1) _returnvalue))
    (bind _returnvalue_3 (+ (`|GetArrayItem` _coords) _returnvalue))
    (`KismetSystemLibrary.DrawDebugArrow` _returnvalue_2 _returnvalue_3 _arrow_size _randomcolour _debugdrawduration _arrow_thickness)
    (bind _returnvalue_4 (+ (`|GetArrayItem` _coords 2) _returnvalue))
    (`KismetSystemLibrary.DrawDebugArrow` _returnvalue_2 _returnvalue_4 _arrow_size _randomcolour _debugdrawduration _arrow_thickness)
    (`KismetSystemLibrary.DrawDebugLine` _returnvalue_3 _returnvalue_4 _randomcolour (`self.debugDrawDuration`) (`self.Arrow Thickness`))))

(fn `Debug_CreateTextAtLocation`
  (params (InputPin :type Text) (InputPin2 :type "Vector Structure") (linearColor :type "LinearColor Structure"))
  (bind _returnvalue (`|SpawnActorFromClass` "/Script/Engine.TextRenderActor" (`KismetMathLibrary.MakeTransform` InputPin2 (struct :`Pitch` 90.0 :`Roll` -90.0)) "Undefined" "MultiplyWithRoot" null null))
  (bind _textrender (`TextRenderActor.TextRender` _returnvalue))
  (`TextRenderComponent.K2_SetText` _textrender InputPin)
  (`TextRenderComponent.SetWorldSize` _textrender 10.0)
  (`TextRenderComponent.SetTextRenderColor` _textrender (`KismetMathLibrary.Conv_LinearColorToColor` linearColor)))

(fn `Debug_DrawCoords`
  (locals (currentX :type Integer) (currentY :type Integer))
  (for _index (range (`self.voxelsCountDepth`))
    (set `local.currentY` _index)
    (for _index_2 (range (`self.voxelsCountWidth`))
      (set `local.currentX` _index_2)
      (bind _worldcoord (`self.Util_IndexesToWorldCoord` (`local.currentX`) (`local.currentY`)))
      (`self.Debug_CreateTextAtLocation` (`KismetTextLibrary.Conv_StringToText` (`KismetStringLibrary.Concat_StrStr` (`KismetStringLibrary.Conv_IntToString` (`local.currentX`)) "," (`KismetStringLibrary.Conv_IntToString` (`local.currentY`)))) _worldcoord))))

(fn `Debug_DrawVoxelGrid`
  (locals (currentY :type Integer) (currentX :type Integer))
  (bind _returnvalue (- (/ (`self.voxelLength`) 2.0) (/ 1.0 2.0)))
  (for _index (range (`self.voxelsCountDepth`))
    (set `local.currentY` _index)
    (for _index_2 (range (`self.voxelsCountWidth`))
      (set `local.currentX` _index_2)
      (bind _worldcoord (`self.Util_IndexesToWorldCoord` (`local.currentX`) (`local.currentY`)))
      (`KismetSystemLibrary.DrawDebugBox` _worldcoord (`KismetMathLibrary.MakeVector` _returnvalue _returnvalue _returnvalue) (struct :`R` 0.776042 :`G` 0.712993 :`B` 0.168752 :`A` 1.0) (struct) (`self.debugDrawDuration`) 1.0))))

(fn `Debug_DrawVoxelHitInformation`
  (params (optionalFilteredCells :type "Array of Boolean"))
  (locals (NewLocalVar :type "LinearColor Structure"))
  (bind _returnvalue (- (- (/ (`self.voxelLength`) 2.0) (/ 2.0 2.0)) 3.0))
  ;[1 0.6395 0.4379] If the filtered cells array was supplied, debug draw that. Otherwise draw the "raw voxel hit data".
  (for (_array_element _array_index) (select `bool` (`KismetArrayLibrary.Array_IsNotEmpty` optionalFilteredCells) :`false` (`self.rawVoxelHitData`) :`true` optionalFilteredCells)
    (bind (_x _y) (`/Game/Classes/BFL_NavMesh.2dArray_1dIndexTo2d` _array_index (`self.voxelsCountWidth`)))
    (bind _worldcoord (`self.Util_IndexesToWorldCoord` _x _y))
    (if _array_element
      ;[0.3874 0.9502 1 1 16] blue = internal cell (NavMesh)
      ; green = was a hit but isn't fully internal
      ; red = wasn't a hit
      (set `local.NewLocalVar` (struct :`G` 0.178287 :`B` 1.0 :`A` 1.0))
      (else
        (set `local.NewLocalVar` (`KismetMathLibrary.SelectColor` (struct :`R` 0.090871 :`G` 1.0 :`B` 0.299864 :`A` 1.0) (struct :`R` 1.0 :`G` 0.159636 :`B` 0.145709 :`A` 1.0) (`|GetArrayItem` (`self.rawVoxelHitData`) _array_index)))))
    (`KismetSystemLibrary.DrawDebugBox` _worldcoord (`KismetMathLibrary.MakeVector` _returnvalue _returnvalue _returnvalue) (`local.NewLocalVar`) (struct) (`self.debugDrawDuration`) 2.0)))

(fn `RunVoxelCollisionChecks`
  (locals (currentX :type Integer) (currentY :type Integer))
  (`|ExecutionSequence`
    (:`then_0`
      (`KismetArrayLibrary.Array_Clear` (`self.rawVoxelHitData`)))
    (:`then_1`
      ;[1 0.627 0.7341] We want to go left to right, then move down a row.
      ; EG [x0, y0] > [x1, y0] > [x2, y0] ... Then [x0, y1]
      ; Outer loop has to be Y (depth), inner loop is X (width)
      (for _index (range (`self.voxelsCountDepth`))
        (set `local.currentY` _index)
        (for _index_2 (range (`self.voxelsCountWidth`))
          (set `local.currentX` _index_2)
          ;[0.5025 1 0.7146] Run overlap check in real world space and record the result.
          (bind _worldcoord (`self.Util_IndexesToWorldCoord` (`local.currentX`) (`local.currentY`)))
          (bind _hitdetected (`self.TestGeometryAtCoord` _worldcoord))
          (`KismetArrayLibrary.Array_Add` (`self.rawVoxelHitData`) _hitdetected))))))

(fn `SetUp`
  (bind _box (`self.Box`))
  (bind (_returnvalue_x _returnvalue_y _returnvalue_z) (`KismetMathLibrary.BreakVector` (`SceneComponent.K2_GetComponentLocation` _box)))
  (bind _returnvalue (/ (`self.voxelLength`) 2.0))
  (bind (_boxextent_x _boxextent_y) (`KismetMathLibrary.BreakVector` (`BoxComponent.BoxExtent` _box)))
  (bind (_boxextent_x_2 _boxextent_y_2) (`KismetMathLibrary.BreakVector` (`BoxComponent.BoxExtent` (`self.Box`))))
  (`|ExecutionSequence`
    (:`then_0`
      ;[1 0.7718 0.7419] Caculate how many cells will be needed. Only looks at X and Y.
      (set `self.voxelsCountWidth` (`KismetMathLibrary.FTrunc` (/ _boxextent_x_2 _returnvalue)))
      (set `self.voxelsCountDepth` (`KismetMathLibrary.FTrunc` (/ _boxextent_y_2 _returnvalue))))
    (:`then_1`
      ;[0.5585 1 0.93] Caclulate our 0,0 position, which we set as top left.
      ; This will be used a lot later when we need to convert relative coords into real world coords.
      (set `self.topLeftCoord` (`KismetMathLibrary.MakeVector` (- _returnvalue_x _boxextent_x) (- _returnvalue_y _boxextent_y) _returnvalue_z)))))

(fn `TestGeometryAtCoord`
  (params (coord :type "Vector Structure"))
  (returns (hitDetected :type Boolean))
  (bind _returnvalue (/ (`self.voxelLength`) 2.0))
  (bind (_outactors _returnvalue_2) (`KismetSystemLibrary.BoxOverlapActors` coord (`KismetMathLibrary.MakeVector` _returnvalue _returnvalue _returnvalue) (`|MakeArray` "ObjectTypeQuery1" :!type "EObjectTypeQuery Enum")))
  (return _returnvalue_2))

(fn `UserConstructionScript`)

(fn `Util_IndexesToWorldCoord`
  (params (xIndex :type Integer) (yIndex :type Integer))
  (returns (worldCoord :type "Vector Structure"))
  (locals (xVoxelAddition :type "Float (double-precision)") (yVoxelAddition :type "Float (double-precision)"))
  (bind (_topleftcoord_x _topleftcoord_y _topleftcoord_z) (`KismetMathLibrary.BreakVector` (`self.topLeftCoord`)))
  (bind _voxellength (`self.voxelLength`))
  (bind _returnvalue (/ (`self.voxelLength`) 2.0))
  (set `local.xVoxelAddition` (* (`KismetMathLibrary.Conv_IntToDouble` xIndex) _voxellength))
  (set `local.yVoxelAddition` (* (`KismetMathLibrary.Conv_IntToDouble` yIndex) _voxellength))
  (return (`KismetMathLibrary.MakeVector` (+ _topleftcoord_x _returnvalue (`local.xVoxelAddition`)) (+ _topleftcoord_y _returnvalue (`local.yVoxelAddition`)) _topleftcoord_z)))

(fn `Util_Vector2dToWorldCoord`
  (params (relativeCoord :type "Vector2D Structure"))
  (returns (worldCoord :type "Vector Structure"))
  (locals (xVoxelAddition :type "Float (double-precision)") (yVoxelAddition :type "Float (double-precision)"))
  (bind (_x _y) (`KismetMathLibrary.BreakVector2D` relativeCoord))
  (bind (_topleftcoord_x _topleftcoord_y _topleftcoord_z) (`KismetMathLibrary.BreakVector` (`self.topLeftCoord`)))
  (bind _voxellength (`self.voxelLength`))
  (bind _returnvalue (/ (`self.voxelLength`) 2.0))
  (set `local.xVoxelAddition` (* _x _voxellength))
  (set `local.yVoxelAddition` (* _y _voxellength))
  (return (`KismetMathLibrary.MakeVector` (+ _topleftcoord_x _returnvalue (`local.xVoxelAddition`)) (+ _topleftcoord_y _returnvalue (`local.yVoxelAddition`)) _topleftcoord_z)))