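; BP_PerimeterMaker traces perimeter outlines from a 2D grid of voxel hit booleans, apparently for NavMesh areas.
; FilterForInternalOnlyCells keeps only cells whose eight neighbours are hits, treating out-of-bounds as hits.
; MakePerimeters gathers directed edges facing four-way misses and recursively links them end-to-start into coordinate chains, marking closed loops complete.
; SimplifyAllChains reduces completed loops to corner points by dropping vertices where the axis of travel does not change.
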(fn `AutoLinkChains`
  (params (baseChain :type "/Game/Structs/ST_CoordChain Structure") (chainTryingToAdd :type "/Game/Structs/ST_CoordChain Structure"))
  (returns (Success :type Boolean) (ST_CoordChain :type "/Game/Structs/ST_CoordChain Structure"))
  (locals (combinedChain :type "/Game/Structs/ST_CoordChain Structure") (baseChainCoordsOnly :type "Array of Vector2D Structure") (incomingChainCoordsOnly :type "Array of Vector2D Structure") (indexToRemove :type Integer))
  (bind _basechaincoordsonly (`local.baseChainCoordsOnly`))
  (bind _incomingchaincoordsonly (`local.incomingChainCoordsOnly`))
  (set `local.baseChainCoordsOnly` (`.coordinates_7_292AFAFC46D8A9CB612BF7A4E4CAFF15` (break `/Game/Structs/ST_CoordChain` baseChain)))
  (set `local.incomingChainCoordsOnly` (`.coordinates_7_292AFAFC46D8A9CB612BF7A4E4CAFF15` (break `/Game/Structs/ST_CoordChain` chainTryingToAdd)))
  (`self.ChainsCanBeLinked` (`local.baseChainCoordsOnly`) (`local.incomingChainCoordsOnly`)
    (:`LinkedForward`
      (`KismetArrayLibrary.Array_Remove` (`local.incomingChainCoordsOnly`))
      (`KismetArrayLibrary.Array_Append` (`local.baseChainCoordsOnly`) (`local.incomingChainCoordsOnly`))
      (return true (make `/Game/Structs/ST_CoordChain` (`local.baseChainCoordsOnly`) (`KismetMathLibrary.EqualExactly_Vector2DVector2D` (`|GetArrayItem` _basechaincoordsonly) (`|GetArrayItem` _basechaincoordsonly (`KismetArrayLibrary.Array_LastIndex` _basechaincoordsonly))))))
    (:`LinkedBackward`
      (`KismetArrayLibrary.Array_Remove` (`local.baseChainCoordsOnly`))
      (`KismetArrayLibrary.Array_Append` (`local.incomingChainCoordsOnly`) (`local.baseChainCoordsOnly`))
      (return true (make `/Game/Structs/ST_CoordChain` (`local.incomingChainCoordsOnly`) (`KismetMathLibrary.EqualExactly_Vector2DVector2D` (`|GetArrayItem` _incomingchaincoordsonly) (`|GetArrayItem` _incomingchaincoordsonly (`KismetArrayLibrary.Array_LastIndex` _incomingchaincoordsonly))))))
    (:`NoLink`
      (return false))))

(fn `CheckNeighbourForHit`
  (params (originalCellX :type Integer) (originalCellY :type Integer) (neighbourOffset :type "/Game/Structs/ST_Directions Structure") (outOfBoundsTreatment :type Boolean))
  (returns (Output :type Boolean))
  (locals (neighbourX :type Integer) (neighbourY :type Integer))
  (bind (_nameforhumans _xdirection _ydirection) (break `/Game/Structs/ST_Directions` neighbourOffset))
  (`|ExecutionSequence`
    (:`then_0`
      ;[0.8853 0.6143 1] calculate the coords of the neighbour cell.
      (set `local.neighbourX` (+ (`local.originalCellX`) _xdirection))
      (set `local.neighbourY` (+ (`local.originalCellY`) _ydirection)))
    (:`then_1`
      (`|ExecutionSequence`
        (:`then_0`
          ;[0.496 0.8691 1] If the neighbour is outside the space, how should we report this?
          ; - if you're checking if this cell is all internal you want all 4 neighbours to be "hits".
          ; - if you're checking for a perimeter you only make them where your neighbour in x direction is a miss.
          ; Therefore user supplies this function "Out of bounds treatment". IE "if the neighbour is out of bounds, treat it as X".
          (if (or (not (`KismetMathLibrary.InRange_IntInt` (`local.neighbourX`) 0 (`self.X Length`) true false)) (not (`KismetMathLibrary.InRange_IntInt` (`local.neighbourY`) 0 (`self.Y Length`) true false)))
            (return (`local.outOfBoundsTreatment`))))
        (:`then_1`
          ;[0.6252 1 0.3659] Neighbour was not OOB. Return if it was a hit or a miss.
          (return (`|GetArrayItem` (`self.voxelHitInformation`) (`self.Util_2dTo1d` (`local.neighbourX`) (`local.neighbourY`)))))))))

(fn `CombineOrPlaceChain`
  (params (IncomingChain :type "/Game/Structs/ST_CoordChain Structure"))
  (locals (chainWasCombined :type Boolean) (index :type Integer) (combinedChainWasCompleted :type Boolean))
  (set `local.chainWasCombined` false)
  (for (_array_element _array_index) (`self.AllChains`)
    (set `local.index` _array_index)
    (bind (_success _st_coordchain) (`self.AutoLinkChains` _array_element (`local.IncomingChain`)))
    (if _success
      (`KismetArrayLibrary.Array_Set` (`self.AllChains`) (`local.index`) _st_coordchain)
      ;[0.5788 1 0.7662 1 16] If this incoming chain was combined then do not try add this incoming chain on to any other chains -> Break.
      ; Also, keep track if this chain combination requires a re-evaluation of all chains or not.
      (set `local.chainWasCombined` true)
      (set `local.combinedChainWasCompleted` (`.complete_6_51B61A1A429C558D239809B6E49FD0AA` (break `/Game/Structs/ST_CoordChain` _st_coordchain)))
      (break)))
  (if (`local.chainWasCombined`)
    ;[1 1 1] If we managed to combine this chain into a pre-existing one. If this didn't "complete" that chain, there is a chance other chains can now be combined.
    (if (not (`local.combinedChainWasCompleted`))
      (`self.TryCombineOustandingChains`))
    (else
      ;[0.5734 1 0.6378] Couldn't combine it with anything pre-existing so we place it as a new chain
      (`KismetArrayLibrary.Array_Add` (`self.AllChains`) (`local.IncomingChain`)))))

(fn `FilterForInternalOnlyCells`
  (locals (oneNeighbourWasMiss :type Boolean) (filteredArray :type "Array of Boolean") (all8Cells :type "Array of /Game/Structs/ST_Directions Structure"))
  (bind _voxelhitinformation (`self.voxelHitInformation`))
  (`KismetArrayLibrary.Array_Resize` (`local.filteredArray`) (`KismetArrayLibrary.Array_Length` _voxelhitinformation))
  (for _index (range (+ (`KismetArrayLibrary.Array_LastIndex` _voxelhitinformation) 1))
    ;[0.6737 1 0.7186] Check up, right, down and left, and all the diagonals. Exit early if one was not a hit.
    (set `local.oneNeighbourWasMiss` false)
    (for _array_element (`local.all8Cells`)
      (bind (_x _y) (`self.Util_1dTo2d` _index))
      (bind _output (`self.CheckNeighbourForHit` _x _y _array_element true))
      (if (not _output)
        (set `local.oneNeighbourWasMiss` true)
        (break)))
    ;[0.4538 0.5566 1 1 14] If there was a neighbour that wasn't a hit then we set "one neighbour was missed" to true. IE true means this cell is not a "full internal" cell
    (`KismetArrayLibrary.Array_Set` (`local.filteredArray`) _index (not (`local.oneNeighbourWasMiss`))))
  ;[1 1 1] Finally, swap in the new, filtered array
  (set `self.voxelHitInformation` (`local.filteredArray`)))

(fn `GetCellsPerimeterContributions`
  (params (xIndex :type Integer) (yIndex :type Integer))
  (returns (permimOne :type Boolean) (coordChainOne :type "/Game/Structs/ST_CoordChain Structure") (perimTwo :type Boolean) (coordChainTwo :type "/Game/Structs/ST_CoordChain Structure"))
  (locals (relativeEdgesBuffer :type "Array of /Game/Structs/ST_RelativeEdgeCoordinates Structure"))
  (bind _relativeedgesbuffer (`local.relativeEdgesBuffer`))
  ;[1 0.1993 0 1 16] NB! We only check for "perimeter contributions" at the edges between cells. We don't check diagonals (like we did when filtering for "internal" cells).
  (for _array_element (`self.DirectionsAndOffsetsReference`)
    ;[1 0.6504 0.9835] If the neighbour was not a hit then we have found part of the perimeter
    (bind _output (`self.CheckNeighbourForHit` (`local.xIndex`) (`local.yIndex`) _array_element))
    (if (not _output)
      ;[1 0.9966 0.577] Make a "relative edge pair of coords"
      (`KismetArrayLibrary.Array_Add` (`local.relativeEdgesBuffer`) (`self.Util_GetRelativeEdgeFromCoordsAndOffset` (`local.xIndex`) (`local.yIndex`) _array_element))))
  (if (`KismetArrayLibrary.Array_IsNotEmpty` _relativeedgesbuffer)
    (bind (_permimone _coordchainone _perimtwo _coordchaintwo) (`self.JoinEdgesOfSingleCell` _relativeedgesbuffer))
    (return _permimone _coordchainone _perimtwo _coordchaintwo)
    (else
      (return false (struct) false))))

(fn `Init`
  (params (arrayXLength :type Integer) (arrayYLength :type Integer) (optionalRawArray :type "Array of Boolean"))
  (returns (success :type Boolean))
  (bind _optionalrawarray (`local.optionalRawArray`))
  (bind _voxelhitinformation (`self.voxelHitInformation`))
  (bind _optionalrawarray_2 (`local.optionalRawArray`))
  (bind _returnvalue (`KismetArrayLibrary.Array_Length` _optionalrawarray))
  (bind _returnvalue_2 (* (`local.arrayXLength`) (`local.arrayYLength`)))
  (`|ExecutionSequence`
    (:`then_0`
      (if (or (<= (`local.arrayYLength`) 0) (<= (`local.arrayXLength`) 0))
        (`KismetSystemLibrary.PrintString` null "Failed to set up array! \nX or Y values supplied both need to be at least 1.")
        (return false)
        (elif (`KismetArrayLibrary.Array_IsNotEmpty` _optionalrawarray)
          (if (!= _returnvalue _returnvalue_2)
            (`KismetSystemLibrary.PrintString` null (`KismetStringLibrary.Concat_StrStr` "Failed to set up array! X multiplied by Y = " (`KismetStringLibrary.Conv_IntToString` _returnvalue_2) " but the length of the array is " (`KismetStringLibrary.Conv_IntToString` _returnvalue) ". "))
            (return false)))))
    (:`then_1`
      (set `self.Y Length` (`local.arrayYLength`))
      (set `self.X Length` (`local.arrayXLength`)))
    (:`then_2`
      (`KismetArrayLibrary.Array_Clear` _voxelhitinformation)
      (`KismetArrayLibrary.Array_Resize` _voxelhitinformation (* (`self.X Length`) (`self.Y Length`)))
      (if (`KismetArrayLibrary.Array_IsNotEmpty` _optionalrawarray_2)
        (set `self.voxelHitInformation` _optionalrawarray_2))
      (return (> (`KismetArrayLibrary.Array_Length` (`self.voxelHitInformation`)) 0)))))

(fn `JoinEdgesOfSingleCell`
  (params (allEdges :type "Array of /Game/Structs/ST_RelativeEdgeCoordinates Structure"))
  (returns (permimOne :type Boolean) (coordChainOne :type "/Game/Structs/ST_CoordChain Structure") (perimTwo :type Boolean) (coordChainTwo :type "/Game/Structs/ST_CoordChain Structure"))
  (locals (individualCoords :type "Array of Vector2D Structure") (listOne :type "Array of Vector2D Structure") (listTwo :type "Array of Vector2D Structure") (currentChainToProcess :type "Array of Vector2D Structure") (NewLocalVar :type Integer))
  (bind _individualcoords (`local.individualCoords`))
  (bind _currentchaintoprocess (`local.currentChainToProcess`))
  (bind _individualcoords_2 (`local.individualCoords`))
  (bind _individualcoords_3 (`local.individualCoords`))
  (bind _individualcoords_4 (`local.individualCoords`))
  (bind _returnvalue (select `int` (`local.NewLocalVar`) :`0` (`local.listOne`) :`1` (`local.listTwo`)))
  (`|ExecutionSequence`
    (:`then_0`
      (for _array_element allEdges
        (bind (_leftcoord _rightcoord) (break `/Game/Structs/ST_RelativeEdgeCoordinates` _array_element))
        (`KismetArrayLibrary.Array_Add` _individualcoords_2 _leftcoord)
        (`KismetArrayLibrary.Array_Add` _individualcoords_2 _rightcoord)))
    (:`then_1`
      (switch `int` (`KismetArrayLibrary.Array_Length` allEdges)
        (:`1`
          (return true (make `/Game/Structs/ST_CoordChain` (`local.individualCoords`)) false))
        (:`2`
          _)
        (:`3`
          _)
        (:`4`
          (for _array_element_2 _individualcoords
            (`KismetArrayLibrary.Array_AddUnique` (`local.listOne`) _array_element_2))
          (`KismetArrayLibrary.Array_Add` (`local.listOne`) (`|GetArrayItem` _individualcoords))
          (return true (make `/Game/Structs/ST_CoordChain` (`local.listOne`) true) false)))
      (while (> (`KismetArrayLibrary.Array_Length` (`local.individualCoords`)) 0)
        (`|ExecutionSequence`
          (:`then_0`
            ;[0.6183 0.7475 1] Get our current edge to process. This is the first to coords in "individual coords". Remove them from the "individual coords" as we are trying to process every item in that list until there are none left.
            (set `local.currentChainToProcess` (`|MakeArray` (`|GetArrayItem` _individualcoords_4) (`|GetArrayItem` _individualcoords_4 1))))
          (:`then_1`
            ;;[0.4912 1 0.8059] Remove the first element twice
            (`KismetArrayLibrary.Array_Remove` _individualcoords_3)
            (`KismetArrayLibrary.Array_Remove` _individualcoords_3))
          (:`then_2`
            (for _index (range 2)
              (set `local.NewLocalVar` _index)
              (if (`KismetArrayLibrary.Array_IsEmpty` (select `int` (`local.NewLocalVar`) :`0` (`local.listOne`) :`1` (`local.listTwo`)))
                (`KismetArrayLibrary.Array_Append` (select `int` (`local.NewLocalVar`) :`0` (`local.listOne`) :`1` (`local.listTwo`)) (`local.currentChainToProcess`))
                (break)
                (else
                  (`self.ChainsCanBeLinked` (select `int` (`local.NewLocalVar`) :`0` (`local.listOne`) :`1` (`local.listTwo`)) (`local.currentChainToProcess`)
                    (:`LinkedForward`
                      (`KismetArrayLibrary.Array_Add` _returnvalue (`|GetArrayItem` _currentchaintoprocess (`KismetArrayLibrary.Array_LastIndex` _currentchaintoprocess)))
                      (break))
                    (:`LinkedBackward`
                      (`KismetArrayLibrary.Array_Insert` _returnvalue (`|GetArrayItem` (`local.currentChainToProcess`)))
                      (break))
                    (:`NoLink`))))))))
      (if (`KismetArrayLibrary.Array_IsEmpty` (`local.listTwo`))
        (return true (make `/Game/Structs/ST_CoordChain` (`local.listOne`)) false)
        (else
          ;[1 1 1 1 12] Last check to see if the lists can be joined together. Required for case A>B, C>D, D>A to create [C,D,A,B] rather than [D,A,B] & [C,D]
          (`self.ChainsCanBeLinked` (`local.listOne`) (`local.listTwo`)
            (:`LinkedBackward`
              ;[1 1 1] Take every element in list one (other than the first, shared element) and add it on to list two.
              (for (_array_element_3 _array_index) (`local.listOne`)
                (if (!= _array_index 0)
                  (`KismetArrayLibrary.Array_Add` (`local.listTwo`) _array_element_3)))
              (return true (make `/Game/Structs/ST_CoordChain` (`local.listTwo`)) false))
            (:`NoLink`
              (return true (make `/Game/Structs/ST_CoordChain` (`local.listOne`)) true (make `/Game/Structs/ST_CoordChain` (`local.listTwo`))))))))))

(fn `MakePerimeters`
  ;[1 1 1] As of 05.11.2024 this function assumes we are working with "full internal" cells only.
  (for _index (range (+ (`KismetArrayLibrary.Array_LastIndex` (`self.voxelHitInformation`)) 1))
    ;[1 0.5752 0.2903 1 15] Only attempt to get perim contribution if this cell is a "hit" and then later filtered down tas a "full internal" cell.
    (if (`|GetArrayItem` (`self.voxelHitInformation`) _index)
      (bind (_x _y) (`self.Util_1dTo2d` _index))
      (bind (_permimone _coordchainone _perimtwo _coordchaintwo) (`self.GetCellsPerimeterContributions` _x _y))
      (if _permimone
        ;[0.6003 1 0.8292 1 16] Combines the chain or places it as a new outstanding chain. If the chain was combined then it will recursively try to combine all oustanding chains as well.
        (`self.CombineOrPlaceChain` _coordchainone)
        (if _perimtwo
          (`self.CombineOrPlaceChain` _coordchaintwo)))))
  (`KismetSystemLibrary.PrintString` null (`KismetStringLibrary.Concat_StrStr` "Found " (`KismetStringLibrary.Conv_IntToString` (`KismetArrayLibrary.Array_Length` (`self.AllChains`))) " chains overall.")))

(fn `SimplifyAllChains`
  (bind _allchains (`self.AllChains`))
  (for _index (range (+ (`KismetArrayLibrary.Array_LastIndex` (`self.AllChains`)) 1))
    (`KismetArrayLibrary.Array_Set` _allchains _index (`self.SimplifyChain` (`|GetArrayItem` _allchains _index)))))

(fn `SimplifyChain`
  (params (chain :type "/Game/Structs/ST_CoordChain Structure"))
  (returns (simplifiedChain :type "/Game/Structs/ST_CoordChain Structure"))
  (locals (axisChange :type "Array of Boolean") (ogCoordChain :type "Array of Vector2D Structure") (simplifiedCoordChain :type "Array of Vector2D Structure") (nextIndex :type Integer))
  (bind (_coordinates _complete) (break `/Game/Structs/ST_CoordChain` chain))
  (bind _ogcoordchain (`local.ogCoordChain`))
  (bind _ogcoordchain_2 (`local.ogCoordChain`))
  (bind _axischange (`local.axisChange`))
  (bind _ogcoordchain_3 (`local.ogCoordChain`))
  (bind _axischange_2 (`local.axisChange`))
  (bind _returnvalue (`KismetArrayLibrary.Array_LastIndex` (`local.ogCoordChain`)))
  (if _complete
    (bind _output_get (set `local.ogCoordChain` _coordinates))
    ;[1 1 1] Remove the last element which is a duplicate of the first.
    (`KismetArrayLibrary.Array_Remove` _ogcoordchain_3 (`KismetArrayLibrary.Array_LastIndex` _ogcoordchain_3))
    ;[1 1 1] Through resizing, all elements will be 0 default. Therefore we only need to write for x changes
    (`KismetArrayLibrary.Array_Resize` (`local.axisChange`) (`KismetArrayLibrary.Array_Length` _output_get))
    (`|ExecutionSequence`
      (:`then_0`
        ;[0.8114 1 0.8614] AxisChange[0] represents the change that takes place to go from coord[0] to [1].
        ; NB: AxisChange.length == Coords.length but we need to consider AxisChange[last element] as unset.
        ;         We will deal with the first and last elements in a special case later.
        (for _index (range (`KismetArrayLibrary.Array_LastIndex` (`local.ogCoordChain`)))
          (if (!= (`KismetMathLibrary.BreakVector2D` (`|GetArrayItem` _ogcoordchain_2 _index)) (`KismetMathLibrary.BreakVector2D` (`|GetArrayItem` _ogcoordchain_2 (+ _index 1))))
            (`KismetArrayLibrary.Array_Set` (`local.axisChange`) _index true)))
        ;[1 1 1] Do same check for the last item.
        (if (!= (`KismetMathLibrary.BreakVector2D` (`|GetArrayItem` _ogcoordchain _returnvalue)) (`KismetMathLibrary.BreakVector2D` (`|GetArrayItem` _ogcoordchain 0)))
          (`KismetArrayLibrary.Array_Set` (`local.axisChange`) _returnvalue true)))
      (:`then_1`
        (`|ExecutionSequence`
          (:`then_0`
            (if (`.complete_6_51B61A1A429C558D239809B6E49FD0AA` (break `/Game/Structs/ST_CoordChain` (`local.chain`)))
              _))
          (:`then_1`
            ;[1 1 1] First index is done separately as it's a special case
            (for _index_2 (range 1 (+ (`KismetArrayLibrary.Array_LastIndex` (`local.axisChange`)) 1))
              ;[1 1 1] If this element's change != last element's change then it is not superflous and we add it to the new chain
              (if (!= (`|GetArrayItem` _axischange_2 (- _index_2 1)) (`|GetArrayItem` _axischange_2 _index_2))
                (`KismetArrayLibrary.Array_Add` (`local.simplifiedCoordChain`) (`|GetArrayItem` (`local.ogCoordChain`) _index_2))))
            (`|ExecutionSequence`
              (:`then_0`
                ;[1 1 1] Do we need the first element?
                (if (!= (`|GetArrayItem` _axischange) (`|GetArrayItem` _axischange (`KismetArrayLibrary.Array_LastIndex` _axischange)))
                  (`KismetArrayLibrary.Array_Insert` (`local.simplifiedCoordChain`) (`|GetArrayItem` (`local.ogCoordChain`)))))
              (:`then_1`
                ;[1 1 1] Return the simplified chain
                (return (make `/Game/Structs/ST_CoordChain` (`local.simplifiedCoordChain`) true))))))))
    (else
      (`KismetSystemLibrary.PrintString` null "Warning: A chain that is not complete attempted to be simplified. The function SimplifyChains only works on completed chains.")
      (return chain))))

(fn `TryCombineOustandingChains`
  (locals (i :type Integer) (j :type Integer) (chainsJoined :type Boolean))
  (bind _chainsjoined (`local.chainsJoined`))
  (set `local.chainsJoined` false)
  (if (< (`KismetArrayLibrary.Array_Length` (`self.AllChains`)) 2)
    (return)
    (else
      (for _index (range (+ (- (`KismetArrayLibrary.Array_Length` (`self.AllChains`)) 2) 1))
        ;[1 0.7285 0.9462 1 15] With this function call, a chain has already been placed. There is no point in continuing, we need to restart. IE we cancel early and recall this same function.
        (if _chainsjoined
          (break)
          (else
            (bind _output_get (set `local.i` _index))
            ;[0.6769 1 0.704 1 16] Skip this chain if it is complete
            (if (not (`.complete_6_51B61A1A429C558D239809B6E49FD0AA` (break `/Game/Structs/ST_CoordChain` (`|GetArrayItem` (`self.AllChains`) _output_get))))
              (for _index_2 (range (+ (`local.i`) 1) (`KismetArrayLibrary.Array_Length` (`self.AllChains`)))
                ;[0.6477 1 0.8182 1 16] Skip this sub chain if it is already complete
                (if (not (`.complete_6_51B61A1A429C558D239809B6E49FD0AA` (break `/Game/Structs/ST_CoordChain` (`|GetArrayItem` (`self.AllChains`)))))
                  (set `local.j` _index_2)
                  (bind (_success _st_coordchain) (`self.AutoLinkChains` (`|GetArrayItem` (`self.AllChains`) (`local.i`)) (`|GetArrayItem` (`self.AllChains`) (`local.j`))))
                  (if _success
                    ;[0.5754 0.7323 1] We need to update one of the chains and delete the other.
                    (`KismetArrayLibrary.Array_Set` (`self.AllChains`) (`local.i`) _st_coordchain)
                    (`KismetArrayLibrary.Array_Remove` (`self.AllChains`) (`local.j`))
                    ;[1 0.5358 0.6179 1 16] Set this to TRUE so we know to break out of this function and start it again
                    (set `local.chainsJoined` true)
                    (break))))))))
      (if _chainsjoined
        (`self.TryCombineOustandingChains`)))))

(fn `Util_1dTo2d`
  (params (`1dIndex` :type Integer))
  (returns (x :type Integer) (y :type Integer))
  (bind _x_length (`self.X Length`))
  (return (mod `1dIndex` _x_length) (/ `1dIndex` _x_length)))

(fn `Util_2dTo1d`
  (params (x :type Integer) (y :type Integer))
  (returns (index :type Integer))
  (return (+ x (* y (`self.X Length`)))))

(fn `Util_GetRelativeEdgeFromCoordsAndOffset`
  (params (x :type Integer) (y :type Integer) (offset :type "/Game/Structs/ST_Directions Structure (by ref)"))
  (returns (offsetEdgeCoords :type "/Game/Structs/ST_RelativeEdgeCoordinates Structure"))
  (bind (_nameforhumans _xdirection _ydirection _pointadjustmentfirst _pointadjustmentsecond) (break `/Game/Structs/ST_Directions` offset))
  (bind (_x _y) (`KismetMathLibrary.BreakVector2D` _pointadjustmentfirst))
  (bind (_x_2 _y_2) (`KismetMathLibrary.BreakVector2D` _pointadjustmentsecond))
  (return (make `/Game/Structs/ST_RelativeEdgeCoordinates` (`KismetMathLibrary.MakeVector2D` (+ x _x) (+ y _y)) (`KismetMathLibrary.MakeVector2D` (+ x _x_2) (+ y _y_2)))))

(fn `Util_Print2dArray`
  (locals (stringInProgress :type String) (overallSummary :type String))
  (bind _x_length (`self.X Length`))
  (for (_array_element _array_index) (`self.voxelHitInformation`)
    (set `local.stringInProgress` (`KismetStringLibrary.Concat_StrStr` (`local.stringInProgress`) (`KismetMathLibrary.SelectString` "1" "0" _array_element) ", "))
    ;[1 1 1] Is this the last element in this row?
    (if (== (mod _array_index _x_length) (- _x_length 1))
      ;[1 1 1] Append this line's summary to overall summary, then reset the line summary
      (set `local.overallSummary` (`KismetStringLibrary.Concat_StrStr` (`local.overallSummary`) " \n" (`local.stringInProgress`)))
      (set `local.stringInProgress` "")))
  (`KismetSystemLibrary.PrintString` null "Summary of 2d array: " true true (struct :`G` 0.66 :`B` 1.0 :`A` 1.0) 10.0)
  (`KismetSystemLibrary.PrintString` null (`local.overallSummary`) true true (struct :`G` 0.66 :`B` 1.0 :`A` 1.0) 10.0))