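; BP_Agent is an actor that travels along an assigned list of 2D waypoints at a set speed.
; AssignWayPoints lifts the points to the actor's current height, precomputes each segment's travel time from distance and speed, then drops the first point as the starting position.
; On Tick, MoveTowardsWayPoint lerps the actor by elapsed time without sweeping, snapping to and removing each waypoint when its time is up.
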(event `self.ReceiveBeginPlay`)

(event `self.ReceiveTick`
  (params (DeltaSeconds :type "Float (single-precision)"))
  (if (> (`KismetArrayLibrary.Array_Length` (`self.Way Points`)) 0)
    (`self.MoveTowardsWayPoint`)))

(fn `AssignWayPoints`
  (params (wayPoints :type "Array of Vector2D Structure"))
  (bind (_returnvalue_x _returnvalue_y _returnvalue_z) (`KismetMathLibrary.BreakVector` (`self.K2_GetActorLocation`)))
  (bind _way_points (`self.Way Points`))
  (bind _way_points_2 (`self.Way Points`))
  (bind _waypointtimings (`self.waypointTimings`))
  (`|ExecutionSequence`
    (:`then_0`
      (`KismetArrayLibrary.Array_Clear` _way_points_2)
      (`KismetArrayLibrary.Array_Resize` _way_points_2 (`KismetArrayLibrary.Array_Length` wayPoints))
      ;[1 1 1] Convert Vector2d into Vector3d
      (for (_array_element _array_index) (`local.wayPoints`)
        (`KismetArrayLibrary.Array_Set` (`self.Way Points`) _array_index (`KismetMathLibrary.Conv_Vector2DToVector` _array_element _returnvalue_z))))
    (:`then_1`
      (`KismetArrayLibrary.Array_Clear` _waypointtimings)
      ;[1 1 1 1 16] We need one fewer since the timings are between points
      (`KismetArrayLibrary.Array_Resize` _waypointtimings (- (`KismetArrayLibrary.Array_Length` (`self.Way Points`)) 1))
      (for (_ _array_index_2) (`self.waypointTimings`)
        (`KismetArrayLibrary.Array_Set` (`self.waypointTimings`) _array_index_2 (/ (`KismetMathLibrary.Vector_Distance` (`|GetArrayItem` _way_points _array_index_2) (`|GetArrayItem` _way_points (+ _array_index_2 1))) (`self.speedUnitsPerSecond`)))))
    (:`then_2`
      ;[1 1 1] Remove element 0 since this is the agent's location already.
      (`KismetArrayLibrary.Array_Remove` (`self.Way Points`)))))

(fn `MoveTowardsWayPoint`
  (bind _way_points (`self.Way Points`))
  (bind _returnvalue (/ (- (`GameplayStatics.GetTimeSeconds`) (`self.timeMarker`)) (`|GetArrayItem` (`self.waypointTimings`))))
  (if (< (`self.timeMarker`) 0.0)
    (if (`KismetArrayLibrary.Array_IsNotEmpty` _way_points) :!label _label
      ;[1 1 1] Prepare for next waypoint
      (set `self.timeMarker` (`GameplayStatics.GetTimeSeconds`))
      (set `self.startPosition` (`self.K2_GetActorLocation`))
      (else
        ;[1 1 1] Reset for future use
        (set `self.timeMarker` -1.0)))
    (elif (> _returnvalue 1.0)
      (`self.K2_SetActorLocation` (`|GetArrayItem` (`self.Way Points`)))
      (`KismetArrayLibrary.Array_Remove` _way_points)
      (`KismetArrayLibrary.Array_Remove` (`self.waypointTimings`))
      (goto _label)
      (else
        (`self.K2_SetActorLocation` (`KismetMathLibrary.VLerp` (`self.startPosition`) (`|GetArrayItem` (`self.Way Points`)) _returnvalue))))))

(fn `UserConstructionScript`)